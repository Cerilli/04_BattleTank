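; Player-controllable tank Blueprint that wires its components together and routes driving, aiming and firing input.
; On BeginPlay it hands the barrel and turret to the aiming component and both tracks to the movement component.
; Movement axes pass intents to the movement component, and Fire calls the aiming component.
; Aim axes rotate the camera rig, splitting yaw onto a gimbal and pitch onto the spring arm.
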(event EventBeginPlay
  (Class|TankAimingComponent|Initialise (Variables|Default|GetTankAiming1) (Variables|Default|GetTankBarrel) (Variables|Default|GetTankTurret))
  (Class|TankMovementComponent|Initialise (Variables|Default|GetTankMovement) (Variables|Default|GetLeftTrack) (Variables|Default|GetRightTrack)))

(event Input|ActionEvents|InputActionFire
  (params (Key :type Key%20Structure))
  ;[1 1 1] Aim Input binding
  (:Pressed
    (Class|TankAimingComponent|Fire (Variables|Default|GetTankAiming1))))

(event Input|AxisEvents|InputAxisAimPitch
  (params (AxisValue :type Float%20%28single-precision%29))
  ;[1 1 1] Aim Input binding
  (Transformation|AddLocalRotation (Variables|Default|GetSpringArm) (Math|Rotator|MakeRotator 0.0 AxisValue 0.0) false false))

(event Input|AxisEvents|InputAxisAimYaw
  (params (AxisValue :type Float%20%28single-precision%29))
  ;[1 1 1] Aim Input binding
  (Transformation|AddLocalRotation (Variables|Default|GetYawGimble) (Math|Rotator|MakeRotator 0.0 0.0 AxisValue) false false))

(event Input|AxisEvents|InputAxisForwardBack
  (params (AxisValue :type Float%20%28single-precision%29))
  ;[1 1 1] Movement
  (Class|TankMovementComponent|IntendMoveForward (Variables|Default|GetTankMovement) AxisValue))

(event Input|AxisEvents|InputAxisTurnRight
  (params (AxisValue :type Float%20%28single-precision%29))
  ;[1 1 1] Movement
  (Class|TankMovementComponent|IntendTurnRight (Variables|Default|GetTankMovement) AxisValue))

(fn ConstructionScript)